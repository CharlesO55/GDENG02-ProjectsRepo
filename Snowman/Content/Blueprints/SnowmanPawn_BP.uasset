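; SnowmanPawn_BP is a player-controlled snowman pawn that handles movement input and hands off control through a PlayerSwitcher.
; MoveX and MoveY axes store clamped values and flags that gate Tick, which adds CalcMoveVec to the first SnowmanPawn_BP's location and sets its own.
; CalcMoveVec's speed- and time-scaled vector math is left unconnected.
; SpaceKey calls SwitchPawn on the switcher, passing itself.
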(event `self.ReceiveTick`
  (params (DeltaSeconds :type "Float (single-precision)"))
  (bind _returnvalue (* (`KismetMathLibrary.MakeVector` (`self.fMoveX`) (`self.fMoveY`)) (`self.SPEED_MULTIPLIER`) DeltaSeconds))
  (if (or (`self.isMoveX`) (`self.isMoveY`))
    (bind _returnvalue_2 (`GameplayStatics.GetActorOfClass` "SnowmanPawn_BP_C"))
    (`KismetSystemLibrary.PrintString` (`KismetStringLibrary.Conv_VectorToString` _returnvalue))
    (`self.K2_SetActorLocation` (+ (`self.K2_GetActorLocation` _returnvalue_2) _returnvalue))))

(event `InputAxis|MoveX`
  (params (AxisValue :type "Float (single-precision)"))
  (bind _output_get (set `self.fMoveX` (`KismetMathLibrary.FClamp` AxisValue -1.0)))
  (set `self.isMoveX` (!= _output_get 0.0)))

(event `InputAction|SpaceKey`
  (params (Key :type "Key Structure"))
  (:`Pressed`
    (bind _asplayer_switcher (cast `PlayerSwitcher` (`self.APlayerSwitcher`)))
    (`PlayerSwitcher.SwitchPawn` _asplayer_switcher self)
    (`KismetSystemLibrary.PrintString` "Blueprint switched out")))

(event `InputAxis|MoveY`
  (params (AxisValue :type "Float (single-precision)"))
  (bind _output_get (set `self.fMoveY` (`KismetMathLibrary.FClamp` AxisValue -1.0)))
  (set `self.isMoveY` (!= _output_get 0.0)))

(fn `UserConstructionScript`)