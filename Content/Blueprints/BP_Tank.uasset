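; BP_Tank is a tank Blueprint that turns its turret and barrel to follow player aim input.
; AimAzimuth yaws an AzimuthBase component and copies its rotation onto the Turret.
; AimElevation pitches the SpringArm within clamped limits, then sets the Barrel pitch from it using a narrower downward, wider upward clamp.
; A disconnected AddLocalRotation path for unclamped elevation remains unused.
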(event `InputAxis|AimElevation`
  (params (AxisValue :type "Float (single-precision)"))
  (bind _barrel (`self.Barrel`))
  (bind _springarm (`self.SpringArm`))
  (bind (_relativerotation_roll _relativerotation_pitch _relativerotation_yaw) (`KismetMathLibrary.BreakRotator` (`SceneComponent.RelativeRotation` _barrel)))
  (bind (_relativerotation_roll_2 _relativerotation_pitch_2) (`KismetMathLibrary.BreakRotator` (`SceneComponent.RelativeRotation` (`self.SpringArm`))))
  (bind (_relativerotation_roll_3 _relativerotation_pitch_3 _relativerotation_yaw_2) (`KismetMathLibrary.BreakRotator` (`SceneComponent.RelativeRotation` _springarm)))
  (`SceneComponent.K2_SetRelativeRotation` _springarm (`KismetMathLibrary.MakeRotator` _relativerotation_roll_3 (`KismetMathLibrary.FClamp` (+ _relativerotation_pitch_3 AxisValue) -89.0 30.0) _relativerotation_yaw_2) false false)
  (`SceneComponent.K2_SetRelativeRotation` _barrel (`KismetMathLibrary.MakeRotator` _relativerotation_roll (`KismetMathLibrary.FClamp` _relativerotation_pitch_2 -5.0 60.0) _relativerotation_yaw) false false))

(event `InputAxis|AimAzimuth`
  (params (AxisValue :type "Float (single-precision)"))
  (bind _azimuthbase (`self.AzimuthBase`))
  (`SceneComponent.K2_AddLocalRotation` _azimuthbase (`KismetMathLibrary.MakeRotator` 0.0 0.0 AxisValue) false false)
  (`SceneComponent.K2_SetRelativeRotation` (`self.Turret`) (`SceneComponent.RelativeRotation` _azimuthbase) false false))

(fn `UserConstructionScript`)