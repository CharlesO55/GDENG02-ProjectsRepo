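; Trigger area actor that despawns poolable actors overlapping it by releasing them back to a coin pool.
; On BeginPlay it caches the PoollingComp from the MGameController reference.
; Each overlap with an ActorPoolable releases it, prints a debug message and refreshes the ScoreHUD coin display with the pool's remaining available size.
; Tick refreshes the same display every frame through UpdateScoreText_2, an identical copy of UpdateScoreText.
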(event `self.ReceiveBeginPlay`
  (set `self.CoinPool` (`self.GetComponentByClass` (`self.m_GameController`) "/Script/CoinPusher.PoollingComp")))

(event `self.ReceiveActorBeginOverlap`
  (params (OtherActor :type "Actor Object Reference"))
  (bind _asactor_poolable (cast `ActorPoolable` OtherActor))
  (`PoollingComp.ReleasePoolable` (`self.CoinPool`) _asactor_poolable)
  (`KismetSystemLibrary.PrintString` (`KismetStringLibrary.Concat_StrStr` "Despawning..." (`KismetSystemLibrary.GetDisplayName` _asactor_poolable)))
  (bind _asscore_hud (cast `/Game/Blueprints/ScoreHUD` (`PlayerController.GetHUD` (`GameplayStatics.GetPlayerController` 0))))
  (bind _returnvalue (`PoollingComp.GetRemainingAvailableSize` (`self.CoinPool`)))
  (`/Game/Blueprints/WB_ScoreUI.UpdateCoinDisplay` (`/Game/Blueprints/ScoreHUD.ScoreUI_Ref` _asscore_hud) (`KismetTextLibrary.Conv_IntToText` _returnvalue)))

(event `self.ReceiveTick`
  (params (DeltaSeconds :type "Float (single-precision)"))
  (bind _asscore_hud (cast `/Game/Blueprints/ScoreHUD` (`PlayerController.GetHUD` (`GameplayStatics.GetPlayerController` 0))))
  (bind _returnvalue (`PoollingComp.GetRemainingAvailableSize` (`self.CoinPool`)))
  (`/Game/Blueprints/WB_ScoreUI.UpdateCoinDisplay` (`/Game/Blueprints/ScoreHUD.ScoreUI_Ref` _asscore_hud) (`KismetTextLibrary.Conv_IntToText` _returnvalue)))

(fn `UserConstructionScript`)