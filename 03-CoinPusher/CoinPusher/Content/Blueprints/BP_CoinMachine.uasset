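; BP_CoinMachine is a coin machine actor that moves a small and a big platform along their relative X axis.
; On BeginPlay it plays the MovePlatformBig timeline, whose two tracks supply an X position for each platform on every update.
; Two helper functions apply those values with SetRelativeLocation, keeping each platform's current Y and Z.
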(event `self.ReceiveBeginPlay`
  (bind _platformsmall (`self.PlatformSmall`))
  (bind _platformbig (`self.PlatformBig`))
  (bind (_relativelocation_x _relativelocation_y _relativelocation_z) (`KismetMathLibrary.BreakVector` (`SceneComponent.RelativeLocation` _platformsmall)))
  (bind (_relativelocation_x_2 _relativelocation_y_2 _relativelocation_z_2) (`KismetMathLibrary.BreakVector` (`SceneComponent.RelativeLocation` _platformbig)))
  (bind (_direction _bigplatformpos _smallplatformpos) (`Timeline|MovePlatformBig`)
    (:`Update`
      (`SceneComponent.K2_SetRelativeLocation` _platformsmall (`KismetMathLibrary.MakeVector` _smallplatformpos _relativelocation_y _relativelocation_z) false false)
      (`SceneComponent.K2_SetRelativeLocation` _platformbig (`KismetMathLibrary.MakeVector` _bigplatformpos _relativelocation_y_2 _relativelocation_z_2) false false))))

(fn `UserConstructionScript`)